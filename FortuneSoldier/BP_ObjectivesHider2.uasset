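; Client-side actor that hides objective icons on the tactical maps in the loadout menu, scoreboard and standalone map.
; It hooks the class-select map toggle, and Tick polls the player's ScoreBoard and Map keybinds.
; These triggers start short-lived looping timers that repeatedly hide icons as widgets load, with the scoreboard handled only once.
; The standalone map is recreated on each open, so its panel is briefly hidden to prevent flicker.
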(event `self.ReceiveBeginPlay`
  ;[0 0 0] Start-up
  ;;[1 0 0] BeginPlay
  (`KismetSystemLibrary.Delay` 1.0)
  (if (not (`KismetSystemLibrary.IsDedicatedServer`))
    (`|ExecutionSequence`
      (:`then_0`
        ;;[0.2344 0.2344 0.2344] Enable tick for ScoreBoard input (only needed on clients/offline)
        (`self.SetActorTickEnabled` true))
      (:`then_1`
        ;[0 0 0] Loadout
        (bind _returnvalue (`KismetSystemLibrary.K2_SetTimerDelegate` (delegate `WaitToLoad`) 0.01 true)))
      (:`then_2`
        (`KismetSystemLibrary.K2_SetTimerDelegate` (`|CreateDelegate` :!event `GetBinds`) 1.0 true)
        (`self.GetBinds`)))))

(event `WaitToLoad`
  ;[0 0 0] Loadout
  (bind _foundwidgets (`WidgetBlueprintLibrary.GetAllWidgetsOfClass` "/Game/UI/Widgets/InGameMenu/ClassSelect/BP_InGameMenu_ClassSelect.BP_InGameMenu_ClassSelect_C" false))
  (if (`KismetArrayLibrary.Array_IsValidIndex` _foundwidgets)
    (add `/Game/UI/Widgets/InGameMenu/ClassSelect/BP_InGameMenu_ClassSelect.OnToggleTacticalMap` (`|GetArrayItem` _foundwidgets) (delegate `Assign_OnTacMapToggle`))
    ;;[0.2344 0.2344 0.2344] Game usually starts on loadout panel
    (`self.Assign_OnTacMapToggle` false)
    (`KismetSystemLibrary.K2_ClearAndInvalidateTimerHandle` (stale `self.ReceiveBeginPlay` _returnvalue))))

(event `Assign_OnTacMapToggle`
  (params (bVisible :type Boolean))
  ;[0 0 0] Loadout
  ;;[0.2344 0.2344 0.2344] Easy method for class selection overviewmap. Binds a delegate removed from a feature to toggle map with button. Could be removed later
  (`KismetSystemLibrary.K2_ClearAndInvalidateTimerHandle` (stale _returnvalue))
  (bind _returnvalue (`KismetSystemLibrary.K2_SetTimerDelegate` (delegate `WaitForObjectiveIcons`) 0.01 true))
  (`KismetSystemLibrary.RetriggerableDelay` 8.0)
  (`KismetSystemLibrary.K2_ClearAndInvalidateTimerHandle` _returnvalue))

(event `WaitForObjectiveIcons`
  ;[0 0 0] Loadout
  ;;[0.2344 0.2344 0.2344] Everytime the loadoutmenu is opened this timer loop is started. Stops a few seconds later
  (bind _returnvalue (`PanelWidget.GetAllChildren` (`TacticalMapWidget.WidgetPanel` (`/Game/UI/Widgets/InGameMenu/ClassSelect/BP_InGameMenu_ClassSelect.MapOverviewWidget` (`|GetArrayItem` (stale `WaitToLoad` _foundwidgets))))))
  (if (`KismetArrayLibrary.Array_IsValidIndex` _returnvalue)
    (for _array_element _returnvalue
      (bind _asobjective_icon (cast `ObjectiveIcon` _array_element))
      ;;;[0.08854 0.08854 0.08854] Hides the objectives
      (`Widget.SetVisibility` _asobjective_icon "Hidden"))))

(event `GetBinds`
  (bind _returnvalue (`INSBlueprintLibrary.GetFirstLocalPlayerController`))
  (bind _returnvalue_2 (`INSBasePlayerController.GetLocalProfile` (`self.LocalPlayer`)))
  ;[0 0 0] Get KeyBinds
  (if (`KismetSystemLibrary.IsValid` _returnvalue)
    (if (not (`KismetSystemLibrary.IsValid` (`self.LocalPlayer`)))
      (bind _asinsplayer_controller (cast `INSPlayerController` _returnvalue))
      (set `self.LocalPlayer` _asinsplayer_controller))
    (bind _keys (`GameInputStatics.GetAllKeysBoundToAction` "ScoreBoard" _returnvalue_2))
    (set `self.ScoreBoardBinds` _keys)
    (bind _keys_2 (`GameInputStatics.GetAllKeysBoundToAction` "Map" _returnvalue_2))
    (set `self.MapBinds` _keys_2)))

(event `self.ReceiveTick`
  (params (DeltaSeconds :type "Float (single-precision)"))
  (bind _localplayer (`self.LocalPlayer`))
  (bind _localplayer_2 (`self.LocalPlayer`))
  ;[0 0 0] Input Tick
  ;;[1 0.02808 0] Tick
  (if (`KismetSystemLibrary.IsValid` (`self.LocalPlayer`))
    (if (not (`self.ScoreboardOpened`))
      (for _array_element (`self.ScoreBoardBinds`)
        ;;[0 0 0] Limits un-needed timer starts. Only works when ther is 1 bind
        (if (`PlayerController.IsInputKeyDown` _localplayer _array_element)
          (`/Engine/EditorBlueprintResources/StandardMacros.DoOnce` false :!label _label
            (:`Completed`
              (`self.OnScoreBoardOpen`)
              (`KismetSystemLibrary.K2_ClearAndInvalidateTimerHandle` (stale _returnvalue))
              (bind _returnvalue (`KismetSystemLibrary.K2_SetTimerDelegate` (`|CreateDelegate` :!event `OnScoreBoardOpen`) 0.01 true))
              ;;[0.1746 0.001821 0.001821] Stop scoreboard tick after done. Remove if needed
              (set `self.ScoreboardOpened` true)
              (`KismetSystemLibrary.RetriggerableDelay` 5.0)
              (`KismetSystemLibrary.K2_ClearAndInvalidateTimerHandle` _returnvalue)))
          (elif (`PlayerController.WasInputKeyJustReleased` _localplayer _array_element)
            (goto _label :!via `Reset`)))))
    (for _array_element_2 (`self.MapBinds`)
      (if (`PlayerController.IsInputKeyDown` _localplayer_2 _array_element_2)
        (`/Engine/EditorBlueprintResources/StandardMacros.DoOnce` false :!label _label_2
          (:`Completed`
            (`self.OnMapOpened`)
            (`self.OnMapLoad`)
            (`KismetSystemLibrary.K2_ClearAndInvalidateTimerHandle` (stale _returnvalue_2))
            (bind _returnvalue_2 (`KismetSystemLibrary.K2_SetTimerDelegate` (`|CreateDelegate` :!event `OnMapOpened`) 0.01 true))
            (`KismetSystemLibrary.RetriggerableDelay` 0.5)
            (`self.OnMapDoneLoad`)
            (`KismetSystemLibrary.RetriggerableDelay` 3.0)
            (`KismetSystemLibrary.K2_ClearAndInvalidateTimerHandle` _returnvalue_2)))
        (elif (`PlayerController.WasInputKeyJustReleased` _localplayer_2 _array_element_2)
          (goto _label_2 :!via `Reset`))))))

(event `OnScoreBoardOpen`
  ;[0 0 0] ScoreBoard
  (bind _foundwidgets (`WidgetBlueprintLibrary.GetAllWidgetsOfClass` "/Game/UI/Widgets/HUD/Scoreboard/BP_Widget_Scoreboard.BP_Widget_Scoreboard_C" false))
  (bind _returnvalue (`PanelWidget.GetAllChildren` (`TacticalMapWidget.WidgetPanel` (`/Game/UI/Widgets/HUD/Scoreboard/BP_Widget_Scoreboard.BP_Widget_TacticalMap_Native` (`|GetArrayItem` _foundwidgets (`KismetArrayLibrary.Array_LastIndex` _foundwidgets))))))
  (if (`KismetArrayLibrary.Array_IsValidIndex` _returnvalue)
    (for _array_element _returnvalue
      (bind _asobjective_icon (cast `ObjectiveIcon` _array_element))
      ;;[0.08854 0.08854 0.08854] Hides the objectives
      (`Widget.SetVisibility` _asobjective_icon "Hidden"))))

(event `OnMapOpened`
  ;[0 0 0] Standalone Map
  (bind _foundwidgets (`WidgetBlueprintLibrary.GetAllWidgetsOfClass` "/Game/UI/Widgets/HUD/TacticalMap/BP_TacticalMap_Standalone.BP_TacticalMap_Standalone_C" false))
  (bind _returnvalue (`PanelWidget.GetAllChildren` (`TacticalMapWidget.WidgetPanel` (`/Game/UI/Widgets/HUD/TacticalMap/BP_TacticalMap_Standalone.BP_Widget_TacticalMap_Native` (`|GetArrayItem` _foundwidgets (`KismetArrayLibrary.Array_LastIndex` _foundwidgets))))))
  (if (`KismetArrayLibrary.Array_IsValidIndex` _returnvalue)
    (for _array_element _returnvalue
      (bind _asobjective_icon (cast `ObjectiveIcon` _array_element))
      ;;[0.08854 0.08854 0.08854] Hides the objectives
      (`Widget.SetVisibility` _asobjective_icon "Hidden"))))

(event `OnMapLoad`
  ;[0 0 0] Fixes flicker for fast loading. Can be used for loadout/scoreboard, but both of those only do it once because they stay loaded. The standalone map is created every input so this is needed.
  (bind _foundwidgets (`WidgetBlueprintLibrary.GetAllWidgetsOfClass` "/Game/UI/Widgets/HUD/TacticalMap/BP_TacticalMap_Standalone.BP_TacticalMap_Standalone_C" false))
  (`Widget.SetVisibility` (`TacticalMapWidget.WidgetPanel` (`/Game/UI/Widgets/HUD/TacticalMap/BP_TacticalMap_Standalone.BP_Widget_TacticalMap_Native` (`|GetArrayItem` _foundwidgets (`KismetArrayLibrary.Array_LastIndex` _foundwidgets)))) "Hidden"))

(event `OnMapDoneLoad`
  ;[0 0 0] Fixes flicker for fast loading. Can be used for loadout/scoreboard, but both of those only do it once because they stay loaded. The standalone map is created every input so this is needed.
  (bind _foundwidgets (`WidgetBlueprintLibrary.GetAllWidgetsOfClass` "/Game/UI/Widgets/HUD/TacticalMap/BP_TacticalMap_Standalone.BP_TacticalMap_Standalone_C" false))
  (`Widget.SetVisibility` (`TacticalMapWidget.WidgetPanel` (`/Game/UI/Widgets/HUD/TacticalMap/BP_TacticalMap_Standalone.BP_Widget_TacticalMap_Native` (`|GetArrayItem` _foundwidgets (`KismetArrayLibrary.Array_LastIndex` _foundwidgets)))) "SelfHitTestInvisible"))

(fn `UserConstructionScript`)