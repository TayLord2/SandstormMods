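; Client-side actor that hides objective icons on the class-select overview map and the scoreboard's tactical map, and disables its tick on dedicated servers.
; It binds to the class-select menu's map-toggle delegate and runs a fast looping timer to hide icons as they load.
; Tick polls the ScoreBoard key bindings until first pressed, then disables itself and starts a similar hiding loop, stopped shortly after icons are found.
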(event `self.ReceiveBeginPlay`
  (`KismetSystemLibrary.Delay` 1.0)
  (if (`KismetSystemLibrary.IsDedicatedServer`)
    ;[0 0 0] Loadout
    ;;[0.2344 0.2344 0.2344] Enable tick for ScoreBoard input (only needed on clients/offline)
    (`self.SetActorTickEnabled` false)
    (else
      (bind _returnvalue (`KismetSystemLibrary.K2_SetTimerDelegate` (delegate `WaitToLoad`) 0.01 true)))))

(event `WaitToLoad`
  ;[0 0 0] Loadout
  (bind _foundwidgets (`WidgetBlueprintLibrary.GetAllWidgetsOfClass` "/Game/UI/Widgets/InGameMenu/ClassSelect/BP_InGameMenu_ClassSelect.BP_InGameMenu_ClassSelect_C" false))
  (if (`KismetArrayLibrary.Array_IsValidIndex` _foundwidgets)
    (add `/Game/UI/Widgets/InGameMenu/ClassSelect/BP_InGameMenu_ClassSelect.OnToggleTacticalMap` (`|GetArrayItem` _foundwidgets) (delegate `Assign_OnTacMapToggle`))
    ;;[0.2344 0.2344 0.2344] Game usually starts on loadout panel
    (`self.Assign_OnTacMapToggle` false)
    (`KismetSystemLibrary.K2_ClearAndInvalidateTimerHandle` (stale `self.ReceiveBeginPlay` _returnvalue))))

(event `Assign_OnTacMapToggle`
  (params (bVisible :type Boolean))
  ;[0 0 0] Loadout
  ;;[0.2344 0.2344 0.2344] Easy method for class selection overviewmap. Uses a delegate removed from a feature to toggle map with button. Could be removed later
  (`KismetSystemLibrary.K2_ClearAndInvalidateTimerHandle` (stale `Assign_OnTacMapToggle` _returnvalue))
  (bind _returnvalue (`KismetSystemLibrary.K2_SetTimerDelegate` (delegate `WaitForObjectiveIcons`) 0.01 true)))

(event `StopLoadOutTimerLoop`
  ;[0 0 0] Loadout
  ;;[0.2344 0.2344 0.2344] Waits a few seconds to disable timer for slow loading
  (`KismetSystemLibrary.K2_ClearAndInvalidateTimerHandle` (stale `Assign_OnTacMapToggle` _returnvalue))
  (goto _label :!via `Reset`))

(event `WaitForObjectiveIcons`
  ;[0 0 0] Loadout
  ;;[0.2344 0.2344 0.2344] Everytime the loadoutmenu is opened this timer loop is started. Stops a few seconds later
  (bind _returnvalue (`PanelWidget.GetAllChildren` (`TacticalMapWidget.WidgetPanel` (`/Game/UI/Widgets/InGameMenu/ClassSelect/BP_InGameMenu_ClassSelect.MapOverviewWidget` (`|GetArrayItem` (stale `WaitToLoad` _foundwidgets))))))
  (if (`KismetArrayLibrary.Array_IsValidIndex` _returnvalue)
    (for _array_element _returnvalue
      (bind _asobjective_icon (cast `ObjectiveIcon` _array_element))
      (`|ExecutionSequence`
        (:`then_0`
          ;;[0.2344 0.2344 0.2344] Waits a few seconds to disable timer for slow loading
          (`/Engine/EditorBlueprintResources/StandardMacros.DoOnce` false :!label _label
            (:`Completed`
              (`KismetSystemLibrary.K2_ClearAndInvalidateTimerHandle` (stale _returnvalue_2))
              (bind _returnvalue_2 (`KismetSystemLibrary.K2_SetTimerDelegate` (delegate `StopLoadOutTimerLoop`) 3.0)))))
        (:`then_1`
          ;;;[0.08854 0.08854 0.08854] Hides the objectives
          (`Widget.SetVisibility` _asobjective_icon "Hidden"))))))

(event `self.ReceiveTick`
  (params (DeltaSeconds :type "Float (single-precision)"))
  (bind _returnvalue (`INSBlueprintLibrary.GetFirstLocalPlayerController`))
  ;[0 0 0] ScoreBoard
  ;;[1 0.02808 0] Tick
  (if (`KismetSystemLibrary.IsValid` _returnvalue)
    (if (not (`KismetSystemLibrary.IsValid` (`self.LocalPlayer`)))
      ;;[0.09375 0.09375 0.09375] Casting can be slow so store it
      (bind _asinsplayer_controller (cast `INSPlayerController` _returnvalue))
      (set `self.LocalPlayer` _asinsplayer_controller))
    ;;[0.1302 0.1302 0.1302] Can be moved to False path (for potential speed gain) but then player can change settings before pressing ScoreBoard inputs to "cheat". You could add another slower timer (1 second etc) to store this as a variable.
    (bind _keys (`GameInputStatics.GetAllKeysBoundToAction` "ScoreBoard" (`INSBasePlayerController.GetLocalProfile` (`self.LocalPlayer`))))
    (for _array_element _keys
      (if (`PlayerController.IsInputKeyDown` (`self.LocalPlayer`) _array_element)
        (`self.OnScoreBoardOpen`)
        (bind _returnvalue_2 (`KismetSystemLibrary.K2_SetTimerDelegate` (delegate `OnScoreBoardOpen`) 0.01 true))
        ;;[0.7969 0.02448 0.01656] Stop the tick. Objective icons could unhide (on scoreboard) at some point. Remove this node to fix.
        (`self.SetActorTickEnabled` false)))))

(event `OnScoreBoardOpen`
  ;[0 0 0] ScoreBoard
  (bind _foundwidgets (`WidgetBlueprintLibrary.GetAllWidgetsOfClass` "/Game/UI/Widgets/HUD/Scoreboard/BP_Widget_Scoreboard.BP_Widget_Scoreboard_C" false))
  (bind _returnvalue (`PanelWidget.GetAllChildren` (`TacticalMapWidget.WidgetPanel` (`/Game/UI/Widgets/HUD/Scoreboard/BP_Widget_Scoreboard.BP_Widget_TacticalMap_Native` (`|GetArrayItem` _foundwidgets)))))
  (if (`KismetArrayLibrary.Array_IsValidIndex` _returnvalue)
    (for _array_element _returnvalue
      (bind _asobjective_icon (cast `ObjectiveIcon` _array_element))
      (`|ExecutionSequence`
        (:`then_0`
          (`/Engine/EditorBlueprintResources/StandardMacros.DoOnce` false :!label _label_2
            (:`Completed`
              (`KismetSystemLibrary.K2_ClearAndInvalidateTimerHandle` (stale _returnvalue_2))
              (bind _returnvalue_2 (`KismetSystemLibrary.K2_SetTimerDelegate` (delegate `DelayedStop`) 2.0)))))
        (:`then_1`
          ;;[0.08854 0.08854 0.08854] Hides the objectives
          (`Widget.SetVisibility` _asobjective_icon "Hidden"))))))

(event `DelayedStop`
  ;[0 0 0] ScoreBoard
  (`KismetSystemLibrary.K2_ClearAndInvalidateTimerHandle` (stale `self.ReceiveTick` _returnvalue_2))
  (goto _label_2 :!via `Reset`))

(fn `UserConstructionScript`)