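; BP_Pickup_MagGrab2 is an actor that, despite its pickup name, holds logic for checking whether a spot is clear of enemy soldiers for spawning.
; On BeginPlay it derives the enemy team, stores a raised spawn location and adds a sphere sized by BotRadius.
; IsSpawnClear returns false if any overlapping pawn is an INSSoldier on the enemy team.
; SelfDestroy removes the actor on authority only.
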(event `self.ReceiveBeginPlay`
  ;[1 1 1] Setup initial vars and set collision sphere to trigger overlaps only for pawns
  (set `self.EnemyTeam` (select `byte` (`self.PlayerTeam`) :`0` 1 :`1` 0 :!type "Byte"))
  (set `self.SpawnLocation` (+ (`self.K2_GetActorLocation` self) (0.0 0.0 180.0)))
  (bind _returnvalue (`AddComponent|NODE_AddSphereComponent-1`))
  (`SphereComponent.SetSphereRadius` _returnvalue (`self.BotRadius`) true))

(fn `Is Spawn Clear?`
  (params (PlayerTeam :type Byte))
  (returns (PointClear :type Boolean))
  (locals (clear :type Boolean))
  (bind _overlappingactors (`self.GetOverlappingActors` self "/Script/Engine.Pawn"))
  (set `self.EnemyTeam` (select `byte` PlayerTeam :`0` 1 :`1` 0 :!type "Byte"))
  (set `local.clear` true)
  (if (> (`KismetArrayLibrary.Array_Length` _overlappingactors) 0)
    (for _array_element _overlappingactors
      (bind _isbot (`self.IsEnemyBot?` _array_element))
      (if _isbot
        (set `local.clear` false))))
  (return (`local.clear`)))

(fn `IsEnemyBot?`
  (params (soldier :type "Actor Object Reference"))
  (returns (IsBot :type Boolean))
  (bind _asinssoldier (cast `INSSoldier` soldier))
  (return (== (`INSSoldier.TeamId` _asinssoldier) (`self.EnemyTeam`))))

(fn `SelfDestroy`
  (`/Engine/EditorBlueprintResources/ActorMacros.Switch Has Authority`
    (:`Authority`
      (`/Engine/EditorBlueprintResources/StandardMacros.IsValid` self
        (:`Is Valid`
          (`self.K2_DestroyActor` self))))))

(fn `UserConstructionScript`)