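; Secondary-slot P90 submachine gun firearm Blueprint that adapts barrel attachment handling to the presence of an underbarrel upgrade.
; It reports the barrel upgrade as movable only when a barrel upgrade is fitted and the underbarrel slot is empty.
; Socket name updates switch the suppressor socket to its elongated variant when an underbarrel is fitted, and back when it is absent.
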(fn `GetMovableUpgrade`
  (returns (ReturnValue :type "WeaponUpgradeComponent Object Reference"))
  (return (`self.GetUpgradeInSlot` "Barrel")))

(fn `HasMovableUpgrade`
  (returns (ReturnValue :type Boolean))
  (return (and (not (`self.HasUpgradeInSlot` "Underbarrel")) (`self.HasUpgradeInSlot` "Barrel"))))

(fn `UpdateSocketName`
  (params (ParentSocket :type Name))
  (returns (ReturnValue :type Name))
  (if (and (== ParentSocket (`KismetStringLibrary.Conv_StringToName` "A_B_Suppressor")) (`self.HasUpgradeInSlot` "Underbarrel"))
    (return (`KismetStringLibrary.Conv_StringToName` "A_B_Suppressor_Elongated"))
    (elif (and (== ParentSocket (`KismetStringLibrary.Conv_StringToName` "A_B_Suppressor_Elongated")) (not (`self.HasUpgradeInSlot` "Underbarrel")))
      (return (`KismetStringLibrary.Conv_StringToName` "A_B_Suppressor")))))

(fn `UserConstructionScript`)