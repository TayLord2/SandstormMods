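; BP_ObjectivesHider is a Blueprint that hides objective-related UI widgets shortly after play begins.
; BeginPlay starts a short timer that re-arms itself a limited number of times, using a counter to stop.
; Each tick of the timer finds all floating objective container, objective dock and active objective display widgets by class and sets them to Hidden.
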(event `self.ReceiveBeginPlay`
  ;[1 0 0] BeginPlay
  (set `self.count` 0)
  (`KismetSystemLibrary.K2_SetTimerDelegate` (delegate `HideStuff`) 2.0 :!label _label))

(event `HideStuff`
  (`self.HideObjectives2`)
  (bind _result (`/Engine/EditorBlueprintResources/StandardMacros.IncrementInt` (`self.count`))
    (:`  `
      (if (< _result 10)
        (goto _label)))))

(event `HideObjectives2`
  (bind _foundwidgets (`WidgetBlueprintLibrary.GetAllWidgetsOfClass` "/Script/Insurgency.FloatingObjectiveContainer" false))
  (`Widget.SetVisibility` _foundwidgets "Hidden")
  (bind _foundwidgets_2 (`WidgetBlueprintLibrary.GetAllWidgetsOfClass` "/Game/UI/Widgets/HUD/BP_ObjectiveDock.BP_ObjectiveDock_C" false))
  (`Widget.SetVisibility` _foundwidgets_2 "Hidden")
  (bind _foundwidgets_3 (`WidgetBlueprintLibrary.GetAllWidgetsOfClass` "/Script/Insurgency.ActiveObjectiveDisplay" false))
  (`Widget.SetVisibility` _foundwidgets_3 "Hidden"))

(fn `UserConstructionScript`)