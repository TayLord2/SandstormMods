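; BP_Hunt_ObjectiveHider is a UI helper actor for the Hunt mode, hiding standard objective widgets and showing hunt-specific information.
; From BeginPlay it re-hides objective docks on a timer for 20 seconds.
; Events display round and crate popups, mark enemies on tactical map and compass, and manage a multiplier HUD created for the owning PlayerController.
; Spawn-icon hiding exists, but its scoreboard delegate binding is unwired.
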(event `RevealEnemies`
  (params (controllers :type "Array of AIController Object Reference") (soldiers :type "Array of INSSoldier Object Reference"))
  (bind _foundwidgets (`WidgetBlueprintLibrary.GetAllWidgetsOfClass` "/Game/UI/Widgets/HUD/TacticalMap/BP_Widget_TacticalMap_Native.BP_Widget_TacticalMap_Native_C" false))
  (for _array_element _foundwidgets
    (for _array_element_2 soldiers
      (bind _returnvalue (`TacticalMapWidget.CreateMapActorWidget` _array_element "/Game/UI/Widgets/HUD/TacticalMap/BP_Widget_TacticalMapPawn.BP_Widget_TacticalMapPawn_C" _array_element_2))
      (`TacticalMapWidget.AddMapActorWidget` _array_element _returnvalue))))

(event `RoundStartedStartup`
  (params (WelcomeText :type Text :default "NSLOCTEXT(\"[CA5DEB6946D24BBA03FC699C6617D1D6]\", \"64BB104E46EADDC83A658AA002EB83F9\", \"<Bold>Hunt</>\\r\\nEliminate all enemies in order to win\")"))
  (bind _foundwidgets (`WidgetBlueprintLibrary.GetAllWidgetsOfClass` "/Game/UI/Widgets/HUD/Multiplayer/BP_MultiplayerGameHUD.BP_MultiplayerGameHUD_C" false))
  (for _array_element _foundwidgets
    (`/Game/UI/Widgets/HUD/Multiplayer/BP_MultiplayerGameHUD.SetCenterPopupMessage` _array_element WelcomeText)))

(event `HighlightEnemyLocation`
  (params (Soldier :type "INSSoldier Object Reference"))
  (bind _foundwidgets (`WidgetBlueprintLibrary.GetAllWidgetsOfClass` "/Game/UI/Widgets/HUD/BP_Compass.BP_Compass_C" false))
  (for _array_element _foundwidgets
    (`/Game/UI/Widgets/HUD/BP_Compass.AddCompassMarkerEvent` _array_element (`self.K2_GetActorLocation` Soldier) Soldier "Danger")))

(event `DisplayCratesLeft`
  (params (CratesLeft :type Integer))
  (bind _foundwidgets (`WidgetBlueprintLibrary.GetAllWidgetsOfClass` "/Game/UI/Widgets/HUD/Multiplayer/BP_MultiplayerGameHUD.BP_MultiplayerGameHUD_C" false))
  (for _array_element _foundwidgets
    (`/Game/UI/Widgets/HUD/Multiplayer/BP_MultiplayerGameHUD.SetCenterPopupMessage` _array_element (`KismetTextLibrary.Conv_StringToText` (`KismetStringLibrary.Concat_StrStr` "Find " (`KismetStringLibrary.Conv_IntToString` CratesLeft) " more crates to unlock crates!")))))

(event `Hide SpawnIcons`
  ;[1 1 1] Hide the faction spawn icons as these are not needed and can overlay the CrateHunt icons
  (bind _foundwidgets (`WidgetBlueprintLibrary.GetAllWidgetsOfClass` "/Game/UI/Widgets/HUD/TacticalMap/BP_Widget_TacticalMapSpawn_Insurgents.BP_Widget_TacticalMapSpawn_Insurgents_C" false))
  (`Widget.SetVisibility` _foundwidgets "Hidden")
  (bind _foundwidgets_2 (`WidgetBlueprintLibrary.GetAllWidgetsOfClass` "/Game/UI/Widgets/HUD/TacticalMap/BP_Widget_TacticalMapSpawn_Insurgents.BP_Widget_TacticalMapSpawn_Insurgents_C" false))
  (`Widget.SetVisibility` _foundwidgets_2 "Hidden"))

(event `OnScoreboardShownDelegate_Event_0`
  (params (bShow :type Boolean))
  ;[1 1 1] Hide the faction spawn icons as these are not needed and can overlay the CrateHunt icons
  (`self.Hide SpawnIcons`))

(event `self.ReceiveBeginPlay`
  (set `self.enable` true)
  (`KismetSystemLibrary.K2_SetTimerDelegate` (delegate `Disable`) 20.0)
  (bind _returnvalue (`KismetSystemLibrary.K2_SetTimerDelegate` (delegate `HideStuff`) 0.5 true :!label _label))
  (set `self.Handle` _returnvalue))

(event `CreateMultipliersHUD`
  ;[1 1 1] Multiplier HUD
  (`KismetSystemLibrary.Delay` 0.2 :!label _label_2)
  (bind _asplayer_controller (cast `PlayerController` (`self.GetOwner`))
    (:`then`
      (if (not (`KismetSystemLibrary.IsDedicatedServer`))
        (bind _returnvalue (`|CreateWidget` "/Hunt/Widgets/HuntHud_Additions.HuntHud_Additions_C" _asplayer_controller))
        (`UserWidget.AddToViewport` _returnvalue -1)
        (bind _output_get (set `self.WidgetHUD` _returnvalue))
        (`/Hunt/Widgets/HuntHud_Additions.FindTeams` _output_get)
        (`/Hunt/Widgets/HuntHud_Additions.UpdateMultiplierCount` _output_get 1.0)))
    (:`CastFailed`
      (goto _label_2))))

(event `Disable`
  (set `self.enable` false))

(event `HideStuff`
  (bind _handle (`self.Handle`))
  (`self.HideObjectives`)
  (if (`self.enable`)
    (goto _label)
    (else
      (`KismetSystemLibrary.K2_PauseTimerHandle` _handle)
      (`KismetSystemLibrary.K2_ClearAndInvalidateTimerHandle` _handle))))

(event `UpdateMultiplierRatio`
  (params (Fraction :type "Float (double-precision)"))
  ;[1 1 1] Multiplier HUD
  (`/Engine/EditorBlueprintResources/StandardMacros.IsValid` (`self.WidgetHUD`)
    (:`Is Valid`
      _)
    (:`Is Not Valid`
      (`self.CreateMultipliersHUD`)))
  (`/Hunt/Widgets/HuntHud_Additions.UpdateMultiplierCount` (`self.WidgetHUD`) Fraction))

(event `RemoveWidget`
  ;[1 1 1] Multiplier HUD
  (`/Hunt/Widgets/HuntHud_Additions.UpdateMultiplierCount` (`self.WidgetHUD`) 0.0) ; Will hide
  (`/Hunt/Widgets/HuntHud_Additions.RemoveAtROundEnd` (`self.WidgetHUD`)))

(event `HideObjectives`
  (bind _foundwidgets (`WidgetBlueprintLibrary.GetAllWidgetsOfClass` "/Game/UI/Widgets/HUD/BP_ObjectiveDock.BP_ObjectiveDock_C" false))
  (`Widget.SetVisibility` _foundwidgets "Hidden")
  (bind _foundwidgets_2 (`WidgetBlueprintLibrary.GetAllWidgetsOfClass` "/Game/UI/Widgets/HUD/BP_ObjectiveDock_CaptureTheBase.BP_ObjectiveDock_CaptureTheBase_C" false))
  (`Widget.SetVisibility` _foundwidgets_2 "Hidden"))

(fn `UserConstructionScript`)