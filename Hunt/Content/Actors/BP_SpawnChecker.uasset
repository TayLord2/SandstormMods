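; Spawn checker actor that reports whether the area around a spawn point is clear of player-team or enemy-team soldiers.
; On BeginPlay it adds a sphere sized by PlayerRadius and derives EnemyTeam from PlayerTeam, while FindTeams can read both from the Checkpoint game mode.
; Query functions filter overlapping INSSoldiers by team ID to return clear flags or an EnemyBots list, which is never emptied here.
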(event `self.ReceiveBeginPlay`
  ;[1 1 1] Setup initial vars and set collision sphere to trigger overlaps only for pawns
  (bind _returnvalue (`AddComponent|NODE_AddSphereComponent-0` :`self` self))
  (`SphereComponent.SetSphereRadius` _returnvalue (`self.PlayerRadius`) true)
  (set `self.EnemyTeam` (select `byte` (`self.PlayerTeam`) :`0` 1 :`1` 0 :!type "Byte")))

(fn `FindTeams`
  (bind _asinscheckpoint_game_mode (cast `INSCheckpointGameMode` (`GameplayStatics.GetGameMode`)))
  (set `self.PlayerTeam` (`INSGameMode.GetAttackingTeam` _asinscheckpoint_game_mode))
  (set `self.EnemyTeam` (`INSGameMode.GetDefendingTeam` _asinscheckpoint_game_mode)))

(fn `GetOverlappingEnemies`
  (returns (Bots :type "Array of INSSoldier Object Reference"))
  (locals (EnemyBots :type "Array of INSSoldier Object Reference"))
  (bind _overlappingactors (`self.GetOverlappingActors` self "/Script/Insurgency.INSSoldier"))
  (if (> (`KismetArrayLibrary.Array_Length` _overlappingactors) 0)
    (for _array_element _overlappingactors
      (bind _asinssoldier (cast `INSSoldier` _array_element))
      (if (== (`INSSoldier.GetTeamId` _asinssoldier) (`self.EnemyTeam`))
        (`KismetArrayLibrary.Array_Add` (`local.EnemyBots`) _asinssoldier)))
    (return (`local.EnemyBots`))
    (else
      (return (`|MakeArray` null :!type "INSSoldier Object Reference")))))

(fn `Is Spawn Clear Of Enemies?`
  (returns (PointClear :type Boolean))
  (locals (Clear :type Boolean))
  (bind _overlappingactors (`self.GetOverlappingActors` self "/Script/Insurgency.INSSoldier"))
  (set `local.Clear` true)
  (if (> (`KismetArrayLibrary.Array_Length` _overlappingactors) 0)
    (for _array_element _overlappingactors
      (bind _asinssoldier (cast `INSSoldier` _array_element))
      (if (== (`INSSoldier.GetTeamId` _asinssoldier) (`self.EnemyTeam`))
        (set `local.Clear` false)
        (break))))
  (return (`local.Clear`)))

(fn `Is Spawn Clear Of Players?`
  (returns (PointClear :type Boolean))
  (locals (Clear :type Boolean))
  (bind _overlappingactors (`self.GetOverlappingActors` self "/Script/Insurgency.INSSoldier"))
  (set `local.Clear` true)
  (if (> (`KismetArrayLibrary.Array_Length` _overlappingactors) 0)
    (for _array_element _overlappingactors
      (bind _asinssoldier (cast `INSSoldier` _array_element))
      (if (== (`INSSoldier.GetTeamId` _asinssoldier) (`self.PlayerTeam`))
        (set `local.Clear` false)
        (break))))
  (return (`local.Clear`)))

(fn `UserConstructionScript`)